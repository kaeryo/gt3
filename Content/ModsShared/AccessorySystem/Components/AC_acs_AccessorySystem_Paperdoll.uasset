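; Accessory system component for a paperdoll that mirrors the accessories of the character it represents.
; On init it sphere-traces around the player for an actor with a matching customization layout, falling back to the player, then copies that AccessoryList and updates visuals.
; A spawned AC_acs_PaperdollMessageProxy relays the source's accessory updates, working around an event binding limitation.
; An older highlight-target lookup remains disconnected.
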(event `self.SystemInit`
  (bind _returnvalue (`GameplayStatics.GetPlayerCharacter` 0))
  (bind _returnvalue_2 (`Actor.K2_GetActorLocation` _returnvalue))
  (if (not (`self.SystemHasInit`))
    (`KismetSystemLibrary.Delay` 0.2)
    (set `self.ActorToCopy` null)
    (`/Engine/EditorBlueprintResources/StandardMacros.IsValid` _returnvalue
      (:`Is Valid`
        (bind (_outhits _returnvalue_3) (`KismetSystemLibrary.SphereTraceMulti` _returnvalue_2 _returnvalue_2 400.0 "TraceTypeQuery1" false (`|MakeArray` (`self.GetOwner`)) "None" false))
        (if _returnvalue_3
          (for _array_element _outhits
            (bind (_bblockinghit _binitialoverlap _time _location _impactpoint _normal _impactnormal _physmat _hitactor) (`GameplayStatics.BreakHitResult` _array_element))
            (if (`KismetStringLibrary.EqualEqual_StrStr` (`CharacterFunctionLibrary.CharacterLayoutToString` (`CharacterCustomizationComponent.Layout` (`Actor.GetComponentByClass` (`self.GetOwner`) "/Game/Characters/BP_CharacterCustomizationComponent.BP_CharacterCustomizationComponent_C"))) (`CharacterFunctionLibrary.CharacterLayoutToString` (`CharacterCustomizationComponent.Layout` (`Actor.GetComponentByClass` _hitactor "/Game/Characters/BP_CharacterCustomizationComponent.BP_CharacterCustomizationComponent_C"))))
              (set `self.ActorToCopy` _hitactor)
              (break)))
          (`/Engine/EditorBlueprintResources/StandardMacros.IsValid` (`self.ActorToCopy`)
            (:`Is Valid`
              _)
            (:`Is Not Valid`
              (set `self.ActorToCopy` (`GameplayStatics.GetPlayerCharacter` 0))))
          (set `self.SystemHasInit` true)
          (`KismetSystemLibrary.Delay` 0.01 :!label _label)
          (set `self.AccessoryList` (`/Game/ModsShared/AccessorySystem/Components/AC_acs_AccessorySystem.AccessoryList` (`Actor.GetComponentByClass` (`self.ActorToCopy`) "/Game/ModsShared/AccessorySystem/Components/AC_acs_AccessorySystem.AC_acs_AccessorySystem_C")))
          (`self.UpdateAccessoryVisuals`)
          ;[1 1 1] Spawning a new component to handle the binding because apparently you can't bind to parent events from other components of the same parent /shrug
          (bind _returnvalue_4 (`FuncomGenericLibrary.AddComponentByClass` (`self.GetOwner`) "/Game/ModsShared/AccessorySystem/Components/AC_acs_PaperdollMessageProxy.AC_acs_PaperdollMessageProxy_C" (`KismetMathLibrary.MakeTransform` (0.0 0.0 0.0))))
          (bind _asac_acs_paperdoll_message_proxy (cast `/Game/ModsShared/AccessorySystem/Components/AC_acs_PaperdollMessageProxy` _returnvalue_4))
          (`/Game/ModsShared/AccessorySystem/Components/AC_acs_PaperdollMessageProxy.SetupMessageProxy` _asac_acs_paperdoll_message_proxy (`self.ActorToCopy`))
          (add `/Game/ModsShared/AccessorySystem/Components/AC_acs_PaperdollMessageProxy.SignalAccessoriesUpdated` _asac_acs_paperdoll_message_proxy (delegate `AccessoriesUpdated`)))))
    (else
      (goto _label))))

(event `AccessoriesUpdated`
  ;[1 1 1] Spawning a new component to handle the binding because apparently you can't bind to parent events from other components of the same parent /shrug
  (set `self.AccessoryList` (`/Game/ModsShared/AccessorySystem/Components/AC_acs_AccessorySystem.AccessoryList` (`Actor.GetComponentByClass` (`self.ActorToCopy`) "/Game/ModsShared/AccessorySystem/Components/AC_acs_AccessorySystem.AC_acs_AccessorySystem_C")))
  (`self.UpdateAccessoryVisuals`))